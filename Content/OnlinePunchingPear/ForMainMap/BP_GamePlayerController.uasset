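; Player controller for the main map of OnlinePunchingPear that handles the in-game menu.
; On BeginPlay it sets game-only input and creates the W_GameMenu widget once, keeping it for reuse.
; Escape calls ToggleGameMenu, which adds or removes the widget and switches between UI-only and game-only input, mouse cursor visibility and the GameMenuIsON flag.
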(event EventBeginPlay
  (Input|SetInputModeGameOnly self)
  (bind _returnvalue (UserInterface|CreateWidget "/Game/OnlinePunchingPear/ForMenuMap/W_GameMenu.W_GameMenu_C"))
  (Variables|Default|SetGameMenuWidget _returnvalue))

(event EventTick
  (params (DeltaSeconds :type Float%20%28single-precision%29)))

(event Input|KeyboardEvents|Escape
  (params (Key :type Key%20Structure :default "None"))
  (:Pressed
    (CallFunction|ToggleGameMenu)))

(fn ConstructionScript)

(fn ToggleGameMenu
  (if (Variables|Default|GetGameMenu_isON?)
    (Widget|RemovefromParent (Variables|Default|GetGameMenuWidget))
    (Input|SetInputModeGameOnly self)
    (Variables|Default|SetbShowMouseCursor false)
    (Variables|Default|SetGameMenu_isON? false)
    (else
      (UserInterface|Viewport|AddtoViewport (Variables|Default|GetGameMenuWidget) 0)
      (Input|SetInputModeUIOnly self (Variables|Default|GetGameMenuWidget) "DoNotLock")
      (Variables|Default|SetbShowMouseCursor true)
      (Variables|Default|SetGameMenu_isON? true))))