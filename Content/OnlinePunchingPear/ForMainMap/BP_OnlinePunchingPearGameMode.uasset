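; Game mode for the OnlinePunchingPear main map that gives each player a separate PlayerStart.
; The ChoosePlayerStart override returns the first PlayerStart not tagged "Taken" and tags it so later players skip it, with no fallback when all are taken.
; The EventGraph holds only disconnected experiments that print start locations and move SpectatorHeadAndBit pawns onto starts, none of which run.
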(fn ConstructionScript)

(fn ChoosePlayerStart
  (params (Player :type Controller%20Object%20Reference))
  ;[1 1 1] Назначение игроков на плеерстарты
  (bind _outactors (Actor|GetAllActorsOfClass "/Script/Engine.PlayerStart"))
  (for _array_element _outactors
    (if (Utilities|Name|NotEqual(Name) (Variables|/Script/Engine.PlayerStart|GetPlayerStartTag _array_element) "Taken")
      (Variables|/Script/Engine.PlayerStart|SetPlayerStartTag _array_element "Taken")
      (return _array_element))))